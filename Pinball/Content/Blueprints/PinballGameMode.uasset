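; Pinball game mode that handles ball respawning, scoring and access to high-score save data.
; It spawns a ball at the first plunger's spawn location and, when that ball is destroyed, spawns another while BallsRemaining is positive, otherwise calling an empty EndGame.
; AddScore applies the Multiplier to incoming points.
; GetSaveGameData lazily caches the HighscoreSave, loading and sorting an existing slot or creating a new object.
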(event Custom|SpawnBall
  (bind _outactors (Actor|GetAllActorsOfClass "/Game/Blueprints/BP_Plunger.BP_Plunger_C"))
  (bind _returnvalue (Game|SpawnActorfromClass "/Game/Blueprints/BP_Ball.BP_Ball_C" (Math|Transform|MakeTransform (Default|GetBallSpawnLocation (Utilities|Array|Get(acopy) _outactors)) "0, 0, 0" "1,1,1") "Undefined" 0 0))
  (Game|BindEventtoOnDestroyed _returnvalue (delegate Custom|OnBallDestroyed)))

(event Custom|OnBallDestroyed
  (params (DestroyedActor :type Actor%20Object%20Reference))
  (if (> (Variables|Default|GetBallsRemaining) 0)
    (CallFunction|SpawnBall)
    (else
      (CallFunction|EndGame))))

(event Custom|EndGame)

(event EventBeginPlay
  (CallFunction|SpawnBall))

(event EventTick
  (params (DeltaSeconds :type Float%20%28single-precision%29)))

(fn ConstructionScript)

(fn AddScore
  (params (PointsToAdd :type Float%20%28single-precision%29))
  (bind _output_get (Variables|Default|SetScore (+ (* PointsToAdd (Variables|Default|GetMultiplier)) (Variables|Default|GetScore))))
  (return _output_get))

(fn GetSaveGameData
  (bind _highscoresavename (Variables|Default|GetHighscoreSaveName))
  (bind _currentsavegameobject (Variables|Default|GetCurrentSaveGameObject)
    (:then
      (return _currentsavegameobject))
    (:else
      (bind _returnvalue (SaveGame|DoesSaveGameExist _highscoresavename))
      (if _returnvalue
        (bind _returnvalue_2 (SaveGame|LoadGamefromSlot _highscoresavename))
        (bind _ashighscore_save (Utilities|Casting|CastToHighscoreSave _returnvalue_2)
          (:then
            (Default|SortSaveData _ashighscore_save)
            (Variables|Default|SetCurrentSaveGameObject _ashighscore_save)
            (return (stale _output_get)))
          (:CastFailed
            _))
        (else
          (bind _returnvalue_3 (SaveGame|CreateSaveGameObject "/Game/Blueprints/HighscoreSave.HighscoreSave_C"))
          (bind _ashighscore_save_2 (Utilities|Casting|CastToHighscoreSave _returnvalue_3)
            (:then
              (bind _output_get (Variables|Default|SetCurrentSaveGameObject _ashighscore_save_2))
              (return _output_get))
            (:CastFailed
              _))))
      (return 0))))